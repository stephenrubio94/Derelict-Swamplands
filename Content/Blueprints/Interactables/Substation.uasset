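; Substation is a repairable interactable device, labeled by its Type enum on a text display and in its mouse-over prompt.
; Interacting needs a Wiring Kit from the player's inventory, which is consumed to mark the device working.
; One Type repairs unconditionally, while all others require their Subsection's PowerStation to be working first.
; Success and failure messages are written to the display through DerelictGameMode.
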(event EventBeginPlay
  (Rendering|Components|TextRender|SetText (Variables|Default|GetDisplayText) (Utilities|Text|ToText(String) (Utilities|String|EnumtoString (Variables|Default|GetType))))
  (Variables|Default|SetMouseOverText (Utilities|Text|ToText(String) (Utilities|String|Append (Utilities|String|EnumtoString (Variables|Default|GetType)) " 
Use Wiring Kit To Repair"))))

(event EventInteract
  (bind _asderelict_character (Utilities|Casting|CastToDerelictCharacter (Game|GetPlayerCharacter 0)))
  (bind _numitems (Default|Get (Variables|/Game/Blueprints/DerelictCharacter.DerelictCharacter_C|GetInventory _asderelict_character) "WiringKit"))
  (if (>= _numitems 1)
    (if (Utilities|Enum|Equal(Enum) (Variables|Default|GetType) "NewEnumerator1")
      (Variables|Default|SetIsWorking true :!label _label)
      (Default|Set (Variables|/Game/Blueprints/DerelictCharacter.DerelictCharacter_C|GetInventory _asderelict_character) "WiringKit" (- _numitems 1))
      (Variables|Default|SetMouseOverText (Utilities|Text|ToText(String) (Utilities|String|Append (Utilities|String|EnumtoString (Variables|Default|GetType)) " 
Working")))
      (bind _asderelict_game_mode (Utilities|Casting|CastToDerelictGameMode (Game|GetGameMode)))
      (Default|WritetoDisplay _asderelict_game_mode "Device Enabled")
      (elif (Variables|Substation_C|GetIsWorking (Variables|/Game/Blueprints/Subsection.Subsection_C|GetPowerStation (Variables|Default|GetSubsection)))
        (goto _label)
        (else
          (bind _asderelict_game_mode_2 (Utilities|Casting|CastToDerelictGameMode (Game|GetGameMode)))
          (Default|WritetoDisplay _asderelict_game_mode_2 "Error: Main Power Disabled"))))
    (else
      (bind _asderelict_game_mode_3 (Utilities|Casting|CastToDerelictGameMode (Game|GetGameMode)))
      (Default|WritetoDisplay _asderelict_game_mode_3 "Wiring Kit Required"))))

(fn ConstructionScript)