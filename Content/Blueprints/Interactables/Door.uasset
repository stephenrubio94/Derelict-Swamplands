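; A door Blueprint that opens on BPOpenDoor and closes itself automatically five seconds later.
; A timeline drives the Door component's relative location by lerping between the DoorClosed and DoorOpen vectors.
; A sequence starts the timeline, then after the delay reverses it, replaying the same open sound for the closing motion.
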(event EventBPOpenDoor
  (Audio|Components|Audio|Play (Variables|Default|GetDoorOpenSound) 0.0)
  (Utilities|FlowControl|Sequence
    (:then_0
      (bind _doorposition (Timeline|DoorOpenTimeline Play)
        (:Update
          (Transformation|SetRelativeLocation (Variables|Default|GetDoor) (Math|Vector|Lerp(Vector) (Variables|Default|GetDoorClosed) (Variables|Default|GetDoorOpen) _doorposition) false false))))
    (:then_1
      (Utilities|FlowControl|Delay 5.0)
      (Audio|Components|Audio|Play (Variables|Default|GetDoorOpenSound) 0.0)
      (Timeline|DoorOpenTimeline Reverse))))

(fn ConstructionScript
  (|CallParentFunction))