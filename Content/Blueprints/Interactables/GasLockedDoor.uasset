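; GasLockedDoor is an interactable door variant that refuses to open while any of its linked gas objects contains gas.
; Its CanOpenDoor override first requires the parent check to pass, then scans LinkedGasObjs and returns false at the first one holding gas.
; A gas block also posts a "Door Disabled, Gas Detected" message through DerelictGameMode, while a failed parent check returns false without that message.
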(event EventBeginPlay)

(event Collision|EventActorBeginOverlap
  (params (OtherActor :type Actor%20Object%20Reference)))

(event EventTick
  (params (DeltaSeconds :type Float%20%28single-precision%29)))

(fn ConstructionScript
  (|CallParentFunction))

(fn CanOpenDoor
  (bind _canopendoor (|CallParentFunction))
  (if _canopendoor
    (for _array_element (Variables|Default|GetLinkedGasObjs)
      (if (Variables|/Game/Blueprints/GasBP.GasBP_C|GetContainsGas _array_element)
        (bind _asderelict_game_mode (Utilities|Casting|CastToDerelictGameMode (Game|GetGameMode)))
        (Default|WritetoDisplay _asderelict_game_mode "" "Door Disabled, Gas Detected")
        (return false)))
    (return true)
    (else
      (return false))))