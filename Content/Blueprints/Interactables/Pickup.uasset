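; Pickup is an interactable item actor that the player collects into their inventory.
; On Interact, it increments its ItemType in the DerelictCharacter's Inventory and plays a 2D pickup sound.
; It then writes a "Picked up" message with the item type name through the DerelictGameMode display and destroys itself.
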(event EventBeginPlay)

(event Collision|EventActorBeginOverlap
  (params (OtherActor :type Actor%20Object%20Reference)))

(event EventTick
  (params (DeltaSeconds :type Float%20%28single-precision%29)))

(event EventInteract
  (bind _asderelict_character (Utilities|Casting|CastToDerelictCharacter (Game|GetPlayerCharacter 0)))
  (Default|Increment (Variables|/Game/Blueprints/DerelictCharacter.DerelictCharacter_C|GetInventory _asderelict_character) (Variables|Default|GetItemType))
  (Audio|PlaySound2D "/Game/Audio/SFX/ItemPickup.ItemPickup")
  (bind _asderelict_game_mode (Utilities|Casting|CastToDerelictGameMode (Game|GetGameMode)))
  (Default|WritetoDisplay _asderelict_game_mode (Utilities|String|Append "Picked up " (Utilities|String|EnumtoString (Variables|Default|GetItemType))))
  (Actor|DestroyActor))

(fn ConstructionScript
  (|CallParentFunction))