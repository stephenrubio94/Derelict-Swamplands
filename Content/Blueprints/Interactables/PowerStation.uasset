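; PowerStation is an interactable Blueprint representing a power station whose type is shown on a display text at BeginPlay.
; Interacting sets IsWorking to true, with a debug print standing in for a planned wiring-kit repair popup.
; One station type branches toward a main-power-disabled error, but its condition is hardcoded true, so that error never occurs.
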(event EventBeginPlay
  (Rendering|Components|TextRender|SetText (Variables|Default|GetDisplayText) (Utilities|Text|ToText(String) (Utilities|String|EnumtoString (Variables|Default|GetType)))))

(event EventInteract
  (Development|PrintString "TODO Popup: do you want to use wiring kit to fix")
  (if (Utilities|Enum|NotEqual(Enum) (Variables|Default|GetType) "NewEnumerator1")
    (Variables|Default|SetIsWorking true :!label _label)
    (elif true
      (goto _label)
      (else
        (Development|PrintString "Error: Main Power Disabled")))))

(fn ConstructionScript)