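; Gas volume for a room that shows fog and flags the player's DerelictCharacter as IsInGas on overlap.
; Every tick it spreads gas in from neighboring gas objects through non-airtight linked doors, and clears it when all doors are airtight and the subsection's AirStation works.
; ContainsGas drives fog visibility, while ChangeGas sets only the fog.
; The player flag is set only when overlap begins in gas and clears when overlap ends.
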(event Custom|ChangeGas
  (params (NewGasStatus :type Boolean))
  (Rendering|SetVisibility (Variables|Default|GetFog) NewGasStatus false))

(event Custom|Update%20Gas%20Status
  (bind _output_get (Variables|Default|SetIsRoomSealed true))
  (for _array_element (Variables|Default|GetLinkedDoors)
    (if (not (Variables|/Script/DerelictSwamplands.Door|GetisAirtight _array_element))
      (Variables|Default|SetIsRoomSealed false)
      (for _array_element_2 (Variables|/Game/Blueprints/Interactables/Door.Door_C|GetLinkedGasObjs _array_element)
        (if (Variables|GasBP_C|GetContainsGas _array_element_2)
          (Variables|Default|SetContainsGas true)))))
  (if _output_get
    (if (Variables|/Game/Blueprints/Interactables/Substation.Substation_C|GetIsWorking (Variables|/Game/Blueprints/Subsection.Subsection_C|GetAirStation (Variables|Default|GetSubsection)))
      (Variables|Default|SetContainsGas false)))
  (Rendering|SetVisibility (Variables|Default|GetFog) (Variables|Default|GetContainsGas) false))

(event Collision|EventActorBeginOverlap
  (params (OtherActor :type Actor%20Object%20Reference))
  (if (Variables|Default|GetContainsGas)
    (bind _asderelict_character (Utilities|Casting|CastToDerelictCharacter (Game|GetPlayerCharacter 0)))
    (Variables|/Script/DerelictSwamplands.DerelictCharacterBase|SetisInGas _asderelict_character true)))

(event Collision|EventActorEndOverlap
  (params (OtherActor :type Actor%20Object%20Reference))
  (bind _asderelict_character (Utilities|Casting|CastToDerelictCharacter (Game|GetPlayerCharacter 0)))
  (Variables|/Script/DerelictSwamplands.DerelictCharacterBase|SetisInGas _asderelict_character false))

(event EventBeginPlay
  (CallFunction|UpdateGasStatus))

(event EventTick
  (params (DeltaSeconds :type Float%20%28single-precision%29))
  (CallFunction|UpdateGasStatus))

(fn ConstructionScript)