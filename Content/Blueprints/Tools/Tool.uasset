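; Base Blueprint for a held tool, with visibility toggling and stub or placeholder actions for use and reload.
; The root component and its children start hidden on BeginPlay and flip visibility when ToggleHolding is called.
; Reload casts to DerelictGameMode and writes the ReloadItem enum name plus "loaded" to its display, while Use is empty.
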(event Custom|Reload
  (bind _asderelict_game_mode (Utilities|Casting|CastToDerelictGameMode (Game|GetGameMode)))
  (Default|WritetoDisplay _asderelict_game_mode (Utilities|String|Append (Utilities|String|EnumtoString (Variables|Default|GetReloadItem)) " loaded")))

(event Custom|Use)

(event Custom|Toggle%20Holding
  (Rendering|ToggleVisibility (Variables|Default|GetDefaultSceneRoot) true))

(event EventBeginPlay
  (Rendering|SetVisibility (Variables|Default|GetDefaultSceneRoot) false true))

(fn ConstructionScript)