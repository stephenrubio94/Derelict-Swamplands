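; Rebreather tool that models a filter wearing down while the device is switched on.
; Each tick while on, it drains the filter duration by a drain rate scaled by delta time.
; Once the filter is depleted, it switches itself off and prints a filter removal message.
; The on/off toggle and filter refill logic exist in the graph but are unwired, so they never run.
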(event EventTick
  (params (DeltaSeconds :type Float%20%28single-precision%29))
  (if (Variables|Default|GetIsOn)
    (if (> (Variables|Default|GetFilterDuration) 0.0)
      (Variables|Default|SetFilterDuration (- (Variables|Default|GetFilterDuration) (* DeltaSeconds (Variables|Default|GetDrainRate))))
      (else
        (Variables|Default|SetIsOn false)
        (Development|PrintString "Removing Filter")))))

(fn ConstructionScript
  (|CallParentFunction))