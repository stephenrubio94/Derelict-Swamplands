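; Blowtorch tool that seals Door actors, using up a load of kerosene per seal.
; The use logic takes a door from the DerelictCharacter's raytrace, seals it if not airtight, and clears Loaded; a separate chain refills it.
; Status messages go to the DerelictGameMode display, and the sparks animation is a TODO print.
; Neither chain has a connected event, so neither runs as shown.
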(fn ConstructionScript)